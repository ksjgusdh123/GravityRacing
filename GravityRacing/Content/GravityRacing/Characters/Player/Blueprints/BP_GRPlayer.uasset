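; BP_GRPlayer is the Gravity Racing player Blueprint, which here handles the handoff from title screen to game UI.
; On BeginPlay it creates the title widget with UI-only input and a hidden cursor, plus a hidden game widget.
; The title widget's start-button callback passes a nickname, which the player stores before hiding the title, switching to game-only input and showing the name on the game widget.
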(event Custom|OnClickedStartButton
  (params (NickName :type Text))
  (bind _gameui (Variables|Default|GetGameUI))
  ;[0.15 0.15 0.15 0.5] Widget
  (Variables|Default|SetName NickName)
  (Widget|SetVisibility (Variables|Default|GetTitleUI) "Hidden")
  (Input|SetInputModeGameOnly (Game|GetPlayerController 0) false)
  (Widget|SetVisibility _gameui "Visible")
  (Default|SetName _gameui (Variables|Default|GetName)))

(event EventBeginPlay
  (bind _returnvalue (Game|GetPlayerController 0))
  (Utilities|FlowControl|Sequence
    (:then_0
      ;[0.15 0.15 0.15 0.5] Widget
      (bind _returnvalue_2 (UserInterface|CreateWidget "/Game/GravityRacing/UI/WBP_Title.WBP_Title_C"))
      (bind _output_get (Variables|Default|SetTitleUI _returnvalue_2))
      (UserInterface|Viewport|AddtoViewport _output_get 0)
      (Input|SetInputModeUIOnly _returnvalue 0 "DoNotLock" false)
      (Variables|/Script/Engine.PlayerController|SetbShowMouseCursor _returnvalue false)
      (EventDispatchers|BindEventtoOnClicked (Variables|Default|GetTitleUI) (delegate Custom|OnClickedStartButton)))
    (:then_1
      (bind _returnvalue_3 (UserInterface|CreateWidget "/Game/GravityRacing/UI/WBP_Game.WBP_Game_C"))
      (bind _output_get_2 (Variables|Default|SetGameUI _returnvalue_3))
      (UserInterface|Viewport|AddtoViewport _output_get_2 0)
      (Widget|SetVisibility (Variables|Default|GetGameUI) "Hidden"))))

(event Collision|EventActorBeginOverlap
  (params (OtherActor :type Actor%20Object%20Reference)))

(event EventTick
  (params (DeltaSeconds :type Float%20%28single-precision%29)))

(fn ConstructionScript)